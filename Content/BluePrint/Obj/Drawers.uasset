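; Drawers actor whose individual drawers the player opens and closes with Interact, with sound and a timeline slide.
; An object trace from the first-person camera picks the static mesh, and its relative X decides whether it slides out or back.
; CanOpen blocks retriggering during the slide.
; The box overlap only shows and hides the prompt widget; input is enabled from BeginPlay, so interaction is not gated by it.
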(event `self.ReceiveBeginPlay`
  (`self.EnableInput` (`GameplayStatics.GetPlayerController` 0))
  (`self.EnableInput` (`GameplayStatics.GetPlayerController` 0))
  (bind _returnvalue (`|CreateWidget` "/Game/BluePrint/Widget/P_Interact.P_Interact_C"))
  (set `self.Interact Prompt` _returnvalue))

(event `InputAction|Interact` :consume false
  (params (Key :type "Key Structure"))
  (bind _returnvalue (`self.K2_GetActorLocation`))
  (bind (_relativelocation_x _relativelocation_y _relativelocation_z) (`KismetMathLibrary.BreakVector` (`SceneComponent.RelativeLocation` (`self.Static Mesh Ref`))))
  (bind (_relativelocation_x_2 _relativelocation_y_2 _relativelocation_z_2) (`KismetMathLibrary.BreakVector` (`SceneComponent.RelativeLocation` (`self.Static Mesh Ref`))))
  (:`Pressed`
    (if (`self.Can Open`)
      (set `self.Can Open` false)
      (bind _asbp_third_person_character (cast `/Game/BluePrint/BP_ThirdPersonCharacter` (`GameplayStatics.GetPlayerCharacter` 0)))
      (bind _fppcamera (`/Game/BluePrint/BP_ThirdPersonCharacter.FPPCamera` _asbp_third_person_character))
      (bind _returnvalue_2 (`SceneComponent.K2_GetComponentLocation` _fppcamera))
      (bind (_outhit _returnvalue_3) (`KismetSystemLibrary.LineTraceSingleForObjects` :`Start` _returnvalue_2 :`End` (+ _returnvalue_2 (* (`SceneComponent.GetForwardVector` _fppcamera) 500.0)) :`ObjectTypes` (`|MakeArray` "ObjectTypeQuery2" :!type "EObjectTypeQuery Enum") :`DrawDebugType` "ForDuration" :`bIgnoreSelf` false))
      (`KismetSystemLibrary.PrintString` (`KismetStringLibrary.Conv_BoolToString` _returnvalue_3))
      (if _returnvalue_3
        (bind (_bblockinghit _binitialoverlap _time _distance _location _impactpoint _normal _impactnormal _physmat _hitactor _hitcomponent) (`GameplayStatics.BreakHitResult` _outhit))
        (bind _asstatic_mesh_component (cast `StaticMeshComponent` _hitcomponent)
          (:`then`
            (`KismetSystemLibrary.PrintString` (`KismetSystemLibrary.GetDisplayName` _hitcomponent))
            (set `self.Static Mesh Ref` _asstatic_mesh_component)
            (bind _relativelocation_x_3 (`KismetMathLibrary.BreakVector` (`SceneComponent.RelativeLocation` _asstatic_mesh_component)))
            (if (not (>= _relativelocation_x_3 25.0))
              (`GameplayStatics.PlaySoundAtLocation` "/Game/Audio/Opening_Drawers.Opening_Drawers" _returnvalue (struct) 0.5 1.0 0.0 null null null null)
              (`KismetSystemLibrary.PrintString` "open")
              (set `self.Start Location` (`KismetMathLibrary.MakeVector` _relativelocation_x _relativelocation_y _relativelocation_z))
              (set `self.End Location` (`KismetMathLibrary.MakeVector` (+ _relativelocation_x 30.0) _relativelocation_y _relativelocation_z))
              (bind (_direction _open_drawer) (`Timeline|Open Drawer`)
                (:`Update`
                  (`SceneComponent.K2_SetRelativeLocation` (`self.Static Mesh Ref`) (`KismetMathLibrary.VLerp` (`self.Start Location`) (`self.End Location`) _open_drawer) false false))
                (:`Finished`
                  (set `self.Can Open` true)))
              (else
                (`GameplayStatics.PlaySoundAtLocation` "/Game/Audio/Closing_Drawers.Closing_Drawers" _returnvalue (struct) 0.5 1.0 0.0 null null null null)
                (set `self.Start Location` (`KismetMathLibrary.MakeVector` _relativelocation_x_2 _relativelocation_y_2 _relativelocation_z_2))
                (set `self.End Location` (`KismetMathLibrary.MakeVector` (+ _relativelocation_x_2 -30.0) _relativelocation_y_2 _relativelocation_z_2))
                (bind (_direction_2 _open_drawer_2) (`Timeline|Timeline_0`)
                  (:`Update`
                    (`SceneComponent.K2_SetRelativeLocation` (`self.Static Mesh Ref`) (`KismetMathLibrary.VLerp` (`self.Start Location`) (`self.End Location`) _open_drawer_2) false false))
                  (:`Finished`
                    (set `self.Can Open` true))))))
          (:`CastFailed`
            (set `self.Can Open` true :!label _label)))
        (else
          (goto _label))))))

(event `self.BoxCollision.OnComponentBeginOverlap`
  (params (OverlappedComponent :type "PrimitiveComponent Object Reference") (OtherActor :type "Actor Object Reference") (OtherComp :type "PrimitiveComponent Object Reference") (OtherBodyIndex :type Integer) (bFromSweep :type Boolean) (SweepResult :type "HitResult Structure (by ref)"))
  (if (== OtherActor (`GameplayStatics.GetPlayerCharacter` 0))
    (`UserWidget.AddToViewport` (`self.Interact Prompt`) 0)
    (cast `/Game/BluePrint/BP_ThirdPersonCharacter` OtherActor)))

(event `self.BoxCollision.OnComponentEndOverlap`
  (params (OverlappedComponent :type "PrimitiveComponent Object Reference") (OtherActor :type "Actor Object Reference") (OtherComp :type "PrimitiveComponent Object Reference") (OtherBodyIndex :type Integer))
  (if (== OtherActor (`GameplayStatics.GetPlayerCharacter` 0))
    (`Widget.RemoveFromParent` (`self.Interact Prompt`))
    (cast `/Game/BluePrint/BP_ThirdPersonCharacter` OtherActor)))

(fn `UserConstructionScript`)