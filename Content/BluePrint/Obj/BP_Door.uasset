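; BP_Door is a door actor that moves vertically when enough pressure switches are active.
; Its activate and deactivate events raise or lower a count of active switches and compare it to the required number.
; Meeting that number plays the DoorActivate timeline, otherwise the timeline reverses, with its track driving the Door component's relative Z location.
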(event `SwtichActivated`
  (bind _pressureswitchactive (`self.PressureSwitchActive`))
  (`/Engine/EditorBlueprintResources/StandardMacros.IncrementInt` _pressureswitchactive
    (:`  `
      (if (>= _pressureswitchactive (`self.PressureSwitchsNeeded`))
        (bind (_direction _newtrack_0) (`Timeline|DoorActivate` :!label _label)
          (:`Update`
            (`SceneComponent.K2_SetRelativeLocation` (`self.Door`) (`KismetMathLibrary.MakeVector` 0.0 0.0 _newtrack_0) false false)))
        (else
          (goto _label :!via `Reverse`))))))

(event `SwtichDeactivated`
  (bind _pressureswitchactive (`self.PressureSwitchActive`))
  (`/Engine/EditorBlueprintResources/StandardMacros.DecrementInt` _pressureswitchactive
    (:`  `
      (if (>= _pressureswitchactive (`self.PressureSwitchsNeeded`))
        (goto _label)
        (else
          (goto _label :!via `Reverse`))))))

(fn `UserConstructionScript`)