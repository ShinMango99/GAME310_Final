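; Interactable door Blueprint that the player swings open and closed with the Interact input while standing near it.
; Overlapping DoorBox shows a P_Interact prompt, enables input and opens a Gate; leaving reverses all three.
; Each press through the Gate runs a FlipFlop that plays or reverses DoorTimeLine.
; The timeline track lerps the Rotate component's yaw to swing the door.
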(event `self.ReceiveBeginPlay`
  (bind _returnvalue (`|CreateWidget` "/Game/BluePrint/Widget/P_Interact.P_Interact_C"))
  (set `self.Interact Prompt` _returnvalue))

(event `InputAction|Interact`
  (params (Key :type "Key Structure"))
  ;[1 1 1] Open n Close the Door
  (:`Pressed`
    (set `self.OpenDoor` true)
    (`/Engine/EditorBlueprintResources/StandardMacros.Gate` true :!label _label
      (:`Exit`
        (if (`self.OpenDoor`)
          (`/Engine/EditorBlueprintResources/StandardMacros.FlipFlop`
            (:`A`
              (bind (_direction _door_track) (`Timeline|Door TimeLine` :!label _label_2)
                (:`Update`
                  (`SceneComponent.K2_SetRelativeRotation` (`self.Rotate`) (`KismetMathLibrary.MakeRotator` 0.0 0.0 (`KismetMathLibrary.Lerp` 0.0 -120.0 _door_track)) false false))))
            (:`B`
              (goto _label_2 :!via `Reverse`)))))))
  (:`Released`
    (set `self.OpenDoor` false)))

(event `self.DoorBox.OnComponentBeginOverlap`
  (params (OverlappedComponent :type "PrimitiveComponent Object Reference") (OtherActor :type "Actor Object Reference") (OtherComp :type "PrimitiveComponent Object Reference") (OtherBodyIndex :type Integer) (bFromSweep :type Boolean) (SweepResult :type "HitResult Structure (by ref)"))
  ;[1 1 1] Open n Close the Door
  (if (== OtherActor (`GameplayStatics.GetPlayerCharacter` 0))
    (`UserWidget.AddToViewport` (`self.Interact Prompt`) 0)
    (bind _asbp_third_person_character (cast `/Game/BluePrint/BP_ThirdPersonCharacter` OtherActor))
    (set `self.Char Ref` _asbp_third_person_character)
    (`self.EnableInput` (`GameplayStatics.GetPlayerController` 0))
    (goto _label :!via `Open`)))

(event `self.DoorBox.OnComponentEndOverlap`
  (params (OverlappedComponent :type "PrimitiveComponent Object Reference") (OtherActor :type "Actor Object Reference") (OtherComp :type "PrimitiveComponent Object Reference") (OtherBodyIndex :type Integer))
  ;[1 1 1] Open n Close the Door
  (if (== OtherActor (`GameplayStatics.GetPlayerCharacter` 0))
    (`Widget.RemoveFromParent` (`self.Interact Prompt`))
    (bind _asbp_third_person_character (cast `/Game/BluePrint/BP_ThirdPersonCharacter` OtherActor))
    (set `self.Char Ref` _asbp_third_person_character)
    (`self.DisableInput` (`GameplayStatics.GetPlayerController` 0))
    (goto _label :!via `Close`)))

(fn `UserConstructionScript`)