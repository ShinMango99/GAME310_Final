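; RockBP is a rock pickup that also makes noise for AI hearing when it hits something.
; A sphere overlap shows an interact prompt and opens a Gate, so pressing Interact increments the character's RockAmount and destroys the rock.
; The first hit on anything but the player passes a DoOnce, playing a sound and reporting a noise event with the player as instigator.
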(event `self.ReceiveBeginPlay`
  ;[1 1 1] Widget
  (`self.EnableInput` (`GameplayStatics.GetPlayerController` 0))
  (bind _returnvalue (`|CreateWidget` "/Game/BluePrint/Widget/P_Interact.P_Interact_C"))
  (set `self.Interact Prompt` _returnvalue))

(event `InputAction|Interact` :consume false
  (params (Key :type "Key Structure"))
  ;[1 1 1] Show the Widget & Pick Up
  (:`Pressed`
    (`/Engine/EditorBlueprintResources/StandardMacros.Gate` true :!label _label
      (:`Exit`
        (bind _result (`/Engine/EditorBlueprintResources/StandardMacros.IncrementInt` (`/Game/BluePrint/BP_ThirdPersonCharacter.Rock Amount` (stale `self.Sphere Collision.OnComponentBeginOverlap` _asbp_third_person_character)))
          (:`  `
            (set `/Game/BluePrint/BP_ThirdPersonCharacter.Rock Amount` _result (stale `self.Sphere Collision.OnComponentBeginOverlap` _asbp_third_person_character))
            (`self.K2_DestroyActor`)))))))

(event `self.Sphere Collision.OnComponentBeginOverlap`
  (params (OverlappedComponent :type "PrimitiveComponent Object Reference") (OtherActor :type "Actor Object Reference") (OtherComp :type "PrimitiveComponent Object Reference") (OtherBodyIndex :type Integer) (bFromSweep :type Boolean) (SweepResult :type "HitResult Structure (by ref)"))
  ;[1 1 1] Show the Widget & Pick Up
  (if (== OtherActor (`GameplayStatics.GetPlayerCharacter` 0))
    (`UserWidget.AddToViewport` (`self.Interact Prompt`) 0)
    (bind _asbp_third_person_character (cast `/Game/BluePrint/BP_ThirdPersonCharacter` OtherActor))
    (goto _label :!via `Open`)))

(event `self.Sphere Collision.OnComponentEndOverlap`
  (params (OverlappedComponent :type "PrimitiveComponent Object Reference") (OtherActor :type "Actor Object Reference") (OtherComp :type "PrimitiveComponent Object Reference") (OtherBodyIndex :type Integer))
  ;[1 1 1] Show the Widget & Pick Up
  (if (== OtherActor (`GameplayStatics.GetPlayerCharacter` 0))
    (`Widget.RemoveFromParent` (`self.Interact Prompt`))
    (cast `/Game/BluePrint/BP_ThirdPersonCharacter` OtherActor)
    (goto _label :!via `Close`)))

(event `self.ReceiveHit`
  (params (MyComp :type "PrimitiveComponent Object Reference") (Other :type "Actor Object Reference") (OtherComp :type "PrimitiveComponent Object Reference") (bSelfMoved :type Boolean) (HitLocation :type "Vector Structure") (HitNormal :type "Vector Structure") (NormalImpulse :type "Vector Structure") (Hit :type "HitResult Structure (by ref)"))
  (bind _returnvalue (`self.K2_GetActorLocation`))
  (bind _returnvalue_2 (`GameplayStatics.GetPlayerCharacter` 0))
  ;[1 1 1] Rock Hit
  (if (!= Other _returnvalue_2)
    (`/Engine/EditorBlueprintResources/StandardMacros.DoOnce` false
      (:`Completed`
        (`GameplayStatics.PlaySoundAtLocation` "/Game/Audio/RockAudioCue.RockAudioCue" _returnvalue (struct) 1.0 1.0 0.0 null null null null)
        (`AISense_Hearing.ReportNoiseEvent` _returnvalue 1.0 _returnvalue_2 3000.0)
        (`KismetSystemLibrary.PrintString` "Hit")))))

(fn `UserConstructionScript`)