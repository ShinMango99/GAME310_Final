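; BP_JumpScare_Trigger02 is a box trigger that fires a one-time jump scare when the player character overlaps it.
; It calls TriggerJumpScareZombie on every ZombieBP in the level, passing the location of the JumpScareEndPointBP03 actor.
; It also plays a loud 2D sting and prints a debug "Hello".
; A near-identical copy of the chain is left unconnected and never runs.
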(event `self.BoxCollision.OnComponentBeginOverlap`
  (params (OverlappedComponent :type "PrimitiveComponent Object Reference") (OtherActor :type "Actor Object Reference") (OtherComp :type "PrimitiveComponent Object Reference") (OtherBodyIndex :type Integer) (bFromSweep :type Boolean) (SweepResult :type "HitResult Structure (by ref)"))
  (cast `/Game/BluePrint/BP_ThirdPersonCharacter` OtherActor)
  (`/Engine/EditorBlueprintResources/StandardMacros.DoOnce` false
    (:`Completed`
      (bind _outactors (`GameplayStatics.GetAllActorsOfClass` "/Game/BluePrint/Animation/ZombieBP.ZombieBP_C"))
      (bind _returnvalue (`GameplayStatics.GetActorOfClass` "/Game/BluePrint/Animation/JumpScareEndPointBP03.JumpScareEndPointBP03_C"))
      (`/Game/BluePrint/Animation/ZombieBP.Trigger JumpScare_Zombie` _outactors (`self.K2_GetActorLocation` _returnvalue))
      (`GameplayStatics.PlaySound2D` "/Game/Audio/jumpscare-sfx.jumpscare-sfx" 2.6 1.0 0.0 null null)
      (`KismetSystemLibrary.PrintString` "Hello"))))

(fn `UserConstructionScript`)