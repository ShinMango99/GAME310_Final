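; Enemy AI that roams at random, chases the player on sight and investigates rock-hit noises.
; PawnSensing starts the chase and audio; a retriggerable delay clears sight, then Tick fades the audio and resumes roaming.
; Roaming moves to random reachable points with random pauses, re-triggered from Tick and move completion.
; AIPerception stimuli from the player send it to the stimulus location, setting an Investigating flag that is never cleared here.
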(event `self.ReceiveBeginPlay`
  ;[1 1 1] Create audio referance
  (bind _returnvalue (`AddComponent|NODE_AddAudioComponent-0`))
  (`AudioComponent.Stop` _returnvalue)
  (set `self.Audio` _returnvalue)
  (`self.Random Roam`))

(event `self.PawnSensing.OnSeePawn`
  (params (Pawn :type "Pawn Object Reference"))
  ;[1 1 1] AI Roam n Chase
  (bind _asbp_third_person_character (cast `/Game/BluePrint/BP_ThirdPersonCharacter` Pawn))
  (`|ExecutionSequence`
    (:`then_0`
      (set `self.Can See Enemy?` true)
      (set `self.isChasing` true)
      (`|AIMoveTo` self (0.0 0.0 0.0) _asbp_third_person_character
        (:`then`
          (`/Engine/EditorBlueprintResources/StandardMacros.DoOnce` false :!label _label
            (:`Completed`
              (`AudioComponent.Play` (`self.Audio`) 0.0))))))
    (:`then_1`
      (`KismetSystemLibrary.RetriggerableDelay` 0.6)
      (set `self.Can See Enemy?` false))))

(event `self.ReceiveTick`
  (params (DeltaSeconds :type "Float (single-precision)"))
  ;[1 1 1] AI Roam n Chase
  (`|ExecutionSequence`
    (:`then_0`
      (if (not (`self.Can See Enemy?`))
        (`KismetSystemLibrary.Delay` 0.4)
        (if (not (`self.Can See Enemy?`))
          (`AudioComponent.FadeOut` (`self.Audio`) 5.0 0.0 "Linear")
          (set `self.isChasing` false)
          (goto _label :!via `Reset`))))
    (:`then_1`
      (if (not (`self.isChasing`))
        (`KismetSystemLibrary.Delay` (`KismetMathLibrary.RandomFloatInRange` 2.0 5.0))
        (`|AIMoveTo` self (`NavigationSystemV1.K2_GetRandomReachablePointInRadius` (`self.K2_GetActorLocation`) 1500.0 null null) null :!label _label_2
          (:`OnSuccess`
            (`KismetSystemLibrary.Delay` (`KismetMathLibrary.RandomFloatInRange` 3.0 7.0)))
          (:`OnFail`
            _))
        (if (not (`self.Investigating`))
          (`self.Random Roam`))))))

(event `Random Roam`
  ;[1 1 1] AI Roam n Chase
  (goto _label_2))

(event `self.AIPerception.OnTargetPerceptionUpdated`
  (params (Actor :type "Actor Object Reference") (Stimulus :type "AIStimulus Structure"))
  (bind (_age _expirationage _strength _stimuluslocation _receiverlocation _tag _bsuccessfullysensed) (break `AIStimulus` Stimulus))
  ;[1 1 1] AI Hearing the Rock hit
  (cast `/Game/BluePrint/BP_ThirdPersonCharacter` Actor)
  (if _bsuccessfullysensed
    (set `self.Investigating` true)
    (`|AIMoveTo` self _stimuluslocation null
      (:`OnSuccess`
        (`KismetSystemLibrary.Delay` 3.0))
      (:`OnFail`
        _))
    (`self.Random Roam`)))

(fn `UserConstructionScript`)