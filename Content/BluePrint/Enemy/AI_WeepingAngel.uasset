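; Enemy AI for AI_WeepingAngel that chases the third-person player character when it detects them directly ahead.
; A self-restarting LookForLight loop box-traces a short distance from the head socket every half second, with debug drawing, and starts AIMoveTo on a player hit.
; A missed trace stops movement; despite the names, no light or gaze check exists.
; PawnSensing's handler is empty, leaving an older distance-limited chase unwired.
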(event `self.PawnSensing.OnSeePawn`
  (params (Pawn :type "Pawn Object Reference")))

(event `self.ReceiveBeginPlay`
  ;[1 1 1] Look 4 Light
  (`self.LookForLight`))

(event `LookForLight`
  (bind _mesh (`self.Mesh`))
  (bind _returnvalue (`SceneComponent.GetSocketLocation` _mesh "head"))
  ;[1 1 1] Look 4 Light
  (`KismetSystemLibrary.Delay` 0.5)
  (set `self.LookTime` (+ 0.5 (`self.LookTime`)))
  (bind (_outhit _returnvalue_2) (`KismetSystemLibrary.BoxTraceSingle` :`Start` _returnvalue :`End` (+ _returnvalue (* (`SceneComponent.GetRightVector` _mesh) 200.0)) :`HalfSize` (10.0 10.0 10.0) :`TraceChannel` "TraceTypeQuery1" :`DrawDebugType` "ForDuration"))
  (if _returnvalue_2
    (set `self.LookTime` 0.0)
    (bind _asbp_third_person_character (cast `/Game/BluePrint/BP_ThirdPersonCharacter` (`.HitActor` (`GameplayStatics.BreakHitResult` _outhit)))
      (:`then`
        (`|AIMoveTo` self (0.0 0.0 0.0) _asbp_third_person_character
          (:`then`
            _)))
      (:`CastFailed`
        _))
    (elif (> (`self.LookTime`) 0.1)
      (`MovementComponent.StopMovementImmediately` (`self.CharacterMovement`))))
  (`self.LookForLight`))

(fn `UserConstructionScript`)