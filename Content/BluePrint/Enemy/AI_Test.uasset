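; Test enemy AI that chases the player character on sight and gives up when the target gets too far away.
; BeginPlay stores the spawn location, and PawnSensing starts an AIMoveTo toward the seen character.
; A delayed polling loop checks distance, then stops movement, pauses and issues a move back to spawn, though that node has no Pawn set.
; The chase move's success and failure only print debug strings.
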(event `self.ReceiveBeginPlay`
  (set `self.SpawnLocation` (`self.K2_GetActorLocation` (`CharacterMovementComponent.GetCharacterOwner` (`self.CharacterMovement`)))))

(event `self.PawnSensing.OnSeePawn`
  (params (Pawn :type "Pawn Object Reference"))
  (bind _asbp_third_person_character (cast `/Game/BluePrint/BP_ThirdPersonCharacter` Pawn))
  (`|AIMoveTo` (`PawnMovementComponent.GetPawnOwner` (`self.CharacterMovement`)) (0.0 0.0 0.0) _asbp_third_person_character
    (:`then`
      (if (> (`self.GetDistanceTo` _asbp_third_person_character) 750.0) :!label _label
        (`MovementComponent.StopMovementImmediately` (`self.CharacterMovement`))
        (`KismetSystemLibrary.Delay` 2.0)
        (`|AIMoveTo` null (`self.SpawnLocation`) null)
        (else
          (`KismetSystemLibrary.Delay` 0.2)
          (goto _label))))
    (:`OnSuccess`
      (`KismetSystemLibrary.PrintString` "1"))
    (:`OnFail`
      (`KismetSystemLibrary.PrintString` "2"))))

(fn `UserConstructionScript`)