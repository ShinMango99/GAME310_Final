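; AI enemy Blueprint that chases the player character when PawnSensing spots it, then returns to its spawn point after losing it.
; Each chase starts a Delay-driven timer loop that halts movement after about two seconds and pauses briefly.
; A box trace from the head socket along the mesh's right vector then decides: hitting the player restarts the chase, while hitting nothing sends the enemy back to its saved spawn location.
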(event `self.ReceiveBeginPlay`
  (set `self.SpawnLocation` (`self.K2_GetActorLocation` (`CharacterMovementComponent.GetCharacterOwner` (`self.CharacterMovement`)))))

(event `self.PawnSensing.OnSeePawn`
  (params (Pawn :type "Pawn Object Reference"))
  (bind _mesh (`self.Mesh`))
  (bind _returnvalue (`SceneComponent.GetSocketLocation` _mesh "head"))
  (bind _returnvalue_2 (`PawnMovementComponent.GetPawnOwner` (`self.CharacterMovement`)))
  (bind _asbp_third_person_character (cast `/Game/BluePrint/BP_ThirdPersonCharacter` Pawn))
  (`|AIMoveTo` _returnvalue_2 (0.0 0.0 0.0) _asbp_third_person_character :!label _label
    (:`then`
      (set `self.FollowTime` (+ (`self.FollowTime`) 0.2) :!label _label_2)
      (if (> (`self.FollowTime`) 2.0)
        (`MovementComponent.StopMovementImmediately` (`self.CharacterMovement`))
        (`KismetSystemLibrary.Delay` 1.0)
        (if true
          (bind (_outhit _returnvalue_3) (`KismetSystemLibrary.BoxTraceSingle` :`Start` _returnvalue :`End` (+ _returnvalue (* (`SceneComponent.GetRightVector` _mesh) 700.0)) :`HalfSize` (10.0 10.0 10.0) :`TraceChannel` "TraceTypeQuery1" :`DrawDebugType` "ForDuration"))
          (if _returnvalue_3
            (cast `/Game/BluePrint/BP_ThirdPersonCharacter` (`.HitActor` (`GameplayStatics.BreakHitResult` _outhit)))
            (set `self.FollowTime` 0.0)
            (goto _label)
            (else
              (`|AIMoveTo` _returnvalue_2 (`self.SpawnLocation`) null
                (:`then`
                  (set `self.FollowTime` 0.0))))))
        (else
          (`KismetSystemLibrary.Delay` 0.2)
          (goto _label_2))))))

(fn `UserConstructionScript`)