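; Battery pickup actor that the player collects by pressing Interact while standing inside its Box trigger.
; It enables player input and creates a P_Interact prompt widget on BeginPlay.
; Player overlap shows or hides the prompt and opens or closes a Gate that filters the Interact press.
; An accepted press calls BatteryPickup on the cached BP_ThirdPersonCharacter, plays the gain sound and destroys the battery.
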(event `self.ReceiveBeginPlay`
  (`self.EnableInput` (`GameplayStatics.GetPlayerController` 0))
  (bind _returnvalue (`|CreateWidget` "/Game/BluePrint/Widget/P_Interact.P_Interact_C"))
  (set `self.Interact Prompt` _returnvalue))

(event `InputAction|Interact` :consume false
  (params (Key :type "Key Structure"))
  ;[1 1 1] Battery PickUp
  (:`Pressed`
    (`/Engine/EditorBlueprintResources/StandardMacros.Gate` true :!label _label
      (:`Exit`
        (`/Game/BluePrint/BP_ThirdPersonCharacter.Battery Pickup` (stale `self.Box.OnComponentBeginOverlap` _asbp_third_person_character))
        (`GameplayStatics.PlaySoundAtLocation` "/Game/Audio/Battery_Gain.Battery_Gain" (`self.K2_GetActorLocation`) (struct) 1.0 1.0 0.0 null null null null)
        (`self.K2_DestroyActor`)))))

(event `self.Box.OnComponentBeginOverlap`
  (params (OverlappedComponent :type "PrimitiveComponent Object Reference") (OtherActor :type "Actor Object Reference") (OtherComp :type "PrimitiveComponent Object Reference") (OtherBodyIndex :type Integer) (bFromSweep :type Boolean) (SweepResult :type "HitResult Structure (by ref)"))
  ;[1 1 1] Battery PickUp
  (if (== OtherActor (`GameplayStatics.GetPlayerCharacter` 0))
    (`UserWidget.AddToViewport` (`self.Interact Prompt`) 0)
    (bind _asbp_third_person_character (cast `/Game/BluePrint/BP_ThirdPersonCharacter` OtherActor))
    (goto _label :!via `Open`)))

(event `self.Box.OnComponentEndOverlap`
  (params (OverlappedComponent :type "PrimitiveComponent Object Reference") (OtherActor :type "Actor Object Reference") (OtherComp :type "PrimitiveComponent Object Reference") (OtherBodyIndex :type Integer))
  ;[1 1 1] Battery PickUp
  (if (== OtherActor (`GameplayStatics.GetPlayerCharacter` 0))
    (`Widget.RemoveFromParent` (`self.Interact Prompt`))
    (cast `/Game/BluePrint/BP_ThirdPersonCharacter` OtherActor)
    (goto _label :!via `Close`)))

(fn `UserConstructionScript`)